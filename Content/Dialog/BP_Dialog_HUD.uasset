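; Dialog controller actor that drives an on-screen UW_Dialog widget from rows in the DialogDT data table.
; ShowDTDialog displays a row by ID as sequential text or a two-option selection, though both options currently read the first response.
; ContinueWithDialog advances text or chains to the chosen response's row, while UpdateIndex moves the highlight.
; Finished rows start quests through AC_QuestManager, sought on the controller for normal dialog but the character for selections.
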(event Custom|ShowDialog
  (params (ID :type Name))
  (CallFunction|ShowDTDialog ID))

(event EventBeginPlay
  (bind _returnvalue (UserInterface|CreateWidget "/Game/Dialog/UW_Dialog.UW_Dialog_C" (Game|GetPlayerController 0)))
  (bind _output_get (Variables|Default|SetDialogWidget _returnvalue))
  (UserInterface|Viewport|AddtoViewport _output_get 0)
  (Widget|SetVisibility _output_get "Hidden"))

(event Collision|EventActorBeginOverlap
  (params (OtherActor :type Actor%20Object%20Reference)))

(event EventTick
  (params (DeltaSeconds :type Float%20%28single-precision%29)))

(fn ConstructionScript)

(fn ShowDTDialog
  (params (ID :type Name))
  (bind _returnvalue (Utilities|GetDataTableRow (Variables|Default|GetDialogDT) ID)
    (:then
      (switch Utilities|FlowControl|Switch|SwitchonE_DialogType (.Type (Utilities|Struct|BreakF_Dialog _returnvalue))
        (:NewEnumerator0
          (bind _output_get (Variables|Default|SetDialogIndex 0))
          (Default|SetNormalDialog (Variables|Default|GetDialogWidget) (Utilities|Text|ToText(String) (Utilities|Array|Get(acopy) (.Texts (Utilities|Struct|BreakF_Dialog _returnvalue)) _output_get)))
          (Widget|SetVisibility (Variables|Default|GetDialogWidget) "Visible")
          (Variables|Default|SetShowingNormalDialog true)
          (Variables|Default|SetCurrentID ID))
        (:NewEnumerator1
          (Variables|Default|SetShowingSelection true)
          (Default|SetSelectionDialog (Variables|Default|GetDialogWidget) (Utilities|Text|ToText(String) (Utilities|Array|Get(acopy) (.Texts (Utilities|Struct|BreakF_Dialog _returnvalue)))) (Utilities|Text|ToText(String) (.text (Utilities|Array|Get(acopy) (.Responses (Utilities|Struct|BreakF_Dialog _returnvalue))))) (Utilities|Text|ToText(String) (.text (Utilities|Array|Get(acopy) (.Responses (Utilities|Struct|BreakF_Dialog _returnvalue))))))
          (Widget|SetVisibility (Variables|Default|GetDialogWidget) "Visible")
          (Variables|Default|SetCurrentID ID))))))

(fn ContinuewithDialog
  (bind _returnvalue (Game|GetPlayerController 0))
  (bind _returnvalue_2 (Game|GetPlayerCharacter 0))
  (bind _returnvalue_3 (Actor|GetComponentbyClass _returnvalue "/Game/Missions/AC_QuestManager.AC_QuestManager_C"))
  (bind _returnvalue_4 (Actor|GetComponentbyClass _returnvalue_2 "/Game/Missions/AC_QuestManager.AC_QuestManager_C"))
  (if (Variables|Default|GetShowingNormalDialog)
    (bind _returnvalue_5 (Utilities|GetDataTableRow (Variables|Default|GetDialogDT) (Variables|Default|GetCurrentID))
      (:then
        (bind _result (Math|Integer|IncrementInt (Variables|Default|GetDialogIndex))
          (:%20%20
            (if (< _result (Utilities|Array|Length (.Texts (Utilities|Struct|BreakF_Dialog _returnvalue_5))))
              (Default|SetNormalDialog (Variables|Default|GetDialogWidget) (Utilities|Text|ToText(String) (Utilities|Array|Get(acopy) (.Texts (Utilities|Struct|BreakF_Dialog _returnvalue_5)) _result)))
              (else
                (Widget|SetVisibility (Variables|Default|GetDialogWidget) "Hidden")
                (Variables|Default|SetCurrentID "None")
                (Variables|Default|SetShowingNormalDialog false)
                (for _array_element (.Quest (Utilities|Struct|BreakF_Dialog _returnvalue_5))
                  (if (!= "" _array_element)
                    (Utilities|IsValid _returnvalue_3
                      (:Is%20Valid
                        (Default|StartQuest _returnvalue_3 _array_element)))))))))))
    (elif (Variables|Default|GetShowingSelection)
      (bind _returnvalue_6 (Utilities|GetDataTableRow (Variables|Default|GetDialogDT) (Variables|Default|GetCurrentID))
        (:then
          (CallFunction|ShowDialog (.id (Utilities|Array|Get(acopy) (.Responses (Utilities|Struct|BreakF_Dialog _returnvalue_6)) (Variables|/Game/Dialog/UW_Dialog.UW_Dialog_C|GetSelectionIndex (Variables|Default|GetDialogWidget)))))
          (for _array_element_2 (.Quest (Utilities|Struct|BreakF_Dialog _returnvalue_6))
            (if (!= _array_element_2 "")
              (Utilities|IsValid _returnvalue_4
                (:Is%20Valid
                  (Default|StartQuest _returnvalue_4 _array_element_2))))))))))

(fn UpdateIndex
  (params (Left :type Boolean))
  (Default|UpdateSelection (Variables|Default|GetDialogWidget) Left))