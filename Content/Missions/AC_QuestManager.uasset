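; Quest manager component that tracks in-progress and completed quests and tests whether a quest can be completed.
; StartQuest updates InProgress and refreshes the quest list on BP_DialogHUD, though it adds "None" instead of the given ID.
; CanComplete reads the Quests data table: Talk requires listed entries in Completed, while Objects counts matching items in the owner's AC_Inventory against a required value.
; CompleteQuest is an empty stub.
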(event EventBeginPlay)

(event EventTick
  (params (DeltaSeconds :type Float%20%28single-precision%29)))

(fn StartQuest
  (params (ID :type Name))
  ;[0.15 0.15 0.15 0.5] Asegurar que no se dupliquen misiones
  (if (!= ID "")
    (Utilities|Array|AddUnique (Variables|Default|GetInProgress) "")
    (bind _asbp_dialog_hud (Utilities|Casting|CastToBP_DialogHUD (HUD|GetHUD (Game|GetPlayerController 0))))
    (Default|UpdateQuests _asbp_dialog_hud)))

(fn CompleteQuest
  (params (ID :type Name)))

(fn CanComplete
  (params (ID :type Name))
  (bind _returnvalue (Components|GetOwner))
  (bind _returnvalue_2 (Actor|GetComponentbyClass _returnvalue "/Game/Inventory/AC_Inventory.AC_Inventory_C"))
  (bind _returnvalue_3 (Utilities|GetDataTableRow (Variables|Default|GetQuests) ID)
    (:then
      (switch Utilities|FlowControl|Switch|SwitchonE_QuestType "NewEnumerator0"
        (:NewEnumerator0
          ;[0.15 0.15 0.15 0.5] Talk Logic
          (LocalVariables|SetCanComplete true)
          (bind _array_element (Utilities|Array|ForEachLoopwithBreak 0 :!label _label)
            (:LoopBody
              (if (not (Utilities|Array|ContainsItem (Variables|Default|GetCompleted) _array_element))
                (LocalVariables|SetCanComplete false)
                (goto _label Break)))
            (:Completed
              (return (LocalVariables|GetCanComplete)))))
        (:NewEnumerator2
          (Utilities|IsValid _returnvalue_2
            (:Is%20Valid
              (LocalVariables|SetNumberOfObjects 0)
              (for _array_element_2 (Variables|/Game/Inventory/AC_Inventory.AC_Inventory_C|GetInventory _returnvalue_2)
                (if (== _array_element_2 (.ObjectName (Utilities|Struct|BreakF_Quest _returnvalue_3)))
                  (Math|Integer|IncrementInt (LocalVariables|GetNumberOfObjects))))
              (return (>= (LocalVariables|GetNumberOfObjects) (.Value (Utilities|Struct|BreakF_Quest _returnvalue_3)))))))))
    (:RowNotFound
      (return false))))